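; Enemy bot that walks forward every tick and smoothly turns toward a stored target rotation.
; NewRotation starts as the spawn rotation, and an accumulated-time throttle gates each small LerpRotator step toward it until within tolerance.
; When life reaches zero, it calls Die on its BotEnemyEasy_Blueprint AI controller, though this check is skipped on ticks where the turn throttle is still accumulating.
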(event `self.ReceiveBeginPlay`
  (set `self.NewRotation` (`self.K2_GetActorRotation`)))

(event `self.ReceiveTick`
  (params (DeltaSeconds :type "Float (single-precision)"))
  (bind _returnvalue (`self.K2_GetActorRotation`))
  (bind _newrotation (`self.NewRotation`))
  (bind _deltasecodsrotation (`self.DeltaSecodsRotation`))
  (`self.WalkForward` (`self.Value Forward`))
  (if (!= _newrotation _returnvalue :`ErrorTolerance` 0.01)
    (bind _output_get (set `self.DeltaSecodsRotation` (+ DeltaSeconds _deltasecodsrotation)))
    (if (>= _output_get 0.01)
      (set `self.DeltaSecodsRotation` 0.0)
      (`self.K2_SetActorRotation` (`KismetMathLibrary.RLerp` _returnvalue _newrotation 0.1))
      (if (<= (`self.GetLife`) 0) :!label _label
        (bind _asbot_enemy_easy_blueprint (cast `/Game/Blueprints/AI/BotEnemyEasy_Blueprint` (`AIBlueprintHelperLibrary.GetAIController` null)))
        (`/Game/Blueprints/AI/BotEnemyEasy_Blueprint.Die` _asbot_enemy_easy_blueprint)))
    (elif (!= _deltasecodsrotation 0.0)
      (set `self.DeltaSecodsRotation` 0.0)
      (goto _label)
      (else
        (goto _label)))))

(fn `UserConstructionScript`)