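; Character Blueprint that switches the player's view to a level camera when the character dies or is destroyed.
; Destroyed, or Tick while GetLife is zero or below, blends player 0's view to the first CameraActor found.
; After a delay, the same chain blends the view back to the character.
; Tick has no one-shot guard, so the camera blend is requested every frame while life stays depleted.
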(event `self.ReceiveDestroyed`
  (bind _returnvalue (`GameplayStatics.GetPlayerController` 0))
  (bind _outactors (`GameplayStatics.GetAllActorsOfClass` "/Script/Engine.CameraActor" :!label _label))
  (`PlayerController.SetViewTargetWithBlend` _returnvalue (`|GetArrayItem` _outactors) 1.0 "VTBlend_Linear" 0.0 false)
  (`KismetSystemLibrary.Delay` 5.0)
  (`PlayerController.SetViewTargetWithBlend` _returnvalue self 1.0 "VTBlend_Linear" 0.0 false))

(event `self.ReceiveTick`
  (params (DeltaSeconds :type "Float (single-precision)"))
  (if (<= (`self.GetLife`) 0)
    (goto _label)))

(fn `UserConstructionScript`)