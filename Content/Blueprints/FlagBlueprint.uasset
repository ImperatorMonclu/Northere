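; Capturable flag that serves as its owner's spawn point and changes hands when another player character or bot overlaps its sphere.
; A capture swaps flags between the old owner and the capturer, then awards score to the capturer.
; SetEntityOwner tints the mesh to the owner's flag color and moves that owner's spawn location to the flag.
; Tick retires the flag once its owner is invalid, clearing the mesh and disabling capture.
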(event `self.Sphere.OnComponentBeginOverlap`
  (params (OverlappedComponent :type "PrimitiveComponent Object Reference") (OtherActor :type "Actor Object Reference") (OtherComp :type "PrimitiveComponent Object Reference") (OtherBodyIndex :type Integer) (bFromSweep :type Boolean) (SweepResult :type "HitResult Structure (by ref)"))
  (bind _entityowner (`self.EntityOwner`))
  (bind _oldowner (`self.OldOwner`))
  (bind _entityowner_2 (`self.EntityOwner`))
  (if (and (`self.IsLife`) (!= OtherActor _entityowner_2) (!= _entityowner_2 (`self.NullOwner`)) (`KismetSystemLibrary.IsValid` _entityowner_2))
    (set `self.OldOwner` (`self.EntityOwner`))
    (bind _asmy_my_character (cast `/Game/Blueprints/MyMyCharacter` OtherActor)
      (:`then`
        (bind _flag (`/Game/Blueprints/MyMyCharacter.Flag` _asmy_my_character))
        (`self.SetEntityOwner` _flag _entityowner)
        (`self.SetEntityOwner` _asmy_my_character)
        (bind _asmy_my_character_2 (cast `/Game/Blueprints/MyMyCharacter` _oldowner)
          (:`then`
            (set `/Game/Blueprints/MyMyCharacter.Flag` _flag _asmy_my_character_2))
          (:`CastFailed`
            (bind _asmy_bot_enemy (cast `/Game/Blueprints/MyBotEnemy` _oldowner))
            (set `/Game/Blueprints/MyBotEnemy.Flag` _flag _asmy_bot_enemy)))
        (set `/Game/Blueprints/MyMyCharacter.Flag` self _asmy_my_character))
      (:`CastFailed`
        (bind _asmy_bot_enemy_2 (cast `/Game/Blueprints/MyBotEnemy` OtherActor))
        (bind _flag_2 (`/Game/Blueprints/MyBotEnemy.Flag` _asmy_bot_enemy_2))
        (`self.SetEntityOwner` _flag_2 _entityowner)
        (`self.SetEntityOwner` _asmy_bot_enemy_2)
        (bind _asmy_my_character_3 (cast `/Game/Blueprints/MyMyCharacter` _oldowner)
          (:`then`
            (set `/Game/Blueprints/MyMyCharacter.Flag` _flag_2 _asmy_my_character_3))
          (:`CastFailed`
            (bind _asmy_bot_enemy_3 (cast `/Game/Blueprints/MyBotEnemy` _oldowner))
            (set `/Game/Blueprints/MyBotEnemy.Flag` _flag_2 _asmy_bot_enemy_3)))
        (set `/Game/Blueprints/MyBotEnemy.Flag` self _asmy_bot_enemy_2)))
    (`Entity.UpdateScore` _entityowner 50)))

(event `self.ReceiveTick`
  (params (DeltaSeconds :type "Float (single-precision)"))
  (bind _entityowner (`self.EntityOwner`))
  (if (not (and (!= _entityowner (`self.NullOwner`)) (`KismetSystemLibrary.IsValid` _entityowner)))
    (`/Engine/EditorBlueprintResources/StandardMacros.DoOnce` false
      (:`Completed`
        (`SkinnedMeshComponent.SetSkinnedAssetAndUpdate` (`self.SkeletalMesh`) null true)
        (set `self.IsLife` false)))))

(fn `SetEntityOwner`
  (params (EntityOwner :type "Entity Object Reference"))
  (set `self.EntityOwner` EntityOwner)
  (`MeshComponent.SetVectorParameterValueOnMaterials` (`self.SkeletalMesh`) "Color" (`KismetMathLibrary.Conv_LinearColorToVector` (`Entity.GetFlagColor` EntityOwner)))
  (`Entity.SetSpawnLocation` EntityOwner (+ (`self.SpawnLocation`) (`self.K2_GetActorLocation`))))

(fn `UserConstructionScript`)