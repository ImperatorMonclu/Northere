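; AI controller for easy enemy bots that sends each toward the nearest living flag it doesn't own and runs the easy behavior tree.
; Perception maintains sensed Entities and writes visibility and the closest target to the Blackboard, alongside ammo state.
; While moving without aiming, a speed-scaled forward sphere trace triggers jumps over obstacles, ignoring Entities and Weapons.
; Death clears Blackboard flags, then reinitializes the bot after a delay.
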(event `self.AIPerception.OnTargetPerceptionUpdated`
  (params (Actor :type "Actor Object Reference") (Stimulus :type "AIStimulus Structure"))
  (bind (_age _expirationage _strength _stimuluslocation _receiverlocation _tag _bsuccessfullysensed) (break `AIStimulus` Stimulus))
  (bind _returnvalue (`AIBlueprintHelperLibrary.GetBlackboard` null))
  (bind _targetentitys (`self.TargetEntitys`))
  (if (> (`Entity.GetLife` (`self.StoredPawn`)) 0)
    (bind _asentity (cast `Entity` Actor))
    (if _bsuccessfullysensed
      (`KismetArrayLibrary.Array_Add` _targetentitys _asentity)
      (`BlackboardComponent.SetValueAsBool` _returnvalue "CanSeeTarget" _bsuccessfullysensed :!label _label)
      (set `self.HowManyNear` 100000000.0 :!label _label_2)
      (for _array_element _targetentitys
        (bind _returnvalue_2 (`KismetMathLibrary.VSize` (- (`self.K2_GetActorLocation` _array_element) (`self.K2_GetActorLocation` (`self.StoredPawn`)))))
        (if (> (`self.HowManyNear`) _returnvalue_2)
          (set `self.TargetEntity` _array_element)
          (set `self.HowManyNear` _returnvalue_2)))
      (`BlackboardComponent.SetValueAsObject` _returnvalue "TargetEntity" (`self.TargetEntity`))
      (elif (`KismetArrayLibrary.Array_Contains` _targetentitys _asentity)
        (`KismetArrayLibrary.Array_RemoveItem` _targetentitys _asentity)
        (if (> (`KismetArrayLibrary.Array_Length` _targetentitys) 0)
          (goto _label_2)
          (else
            (goto _label)))))))

(event `BeginPlayBot`
  (params (MyBot :type "/Game/Blueprints/MyBotEnemy Object Reference"))
  (bind _flagtarget (`self.FlagTarget`))
  (bind _outactors (`GameplayStatics.GetAllActorsOfClass` "/Game/Blueprints/FlagBlueprint.FlagBlueprint_C"))
  (for _array_element _outactors
    (if (and (!= (`/Game/Blueprints/FlagBlueprint.EntityOwner` _array_element) MyBot) (`/Game/Blueprints/FlagBlueprint.IsLife` _array_element))
      (`KismetArrayLibrary.Array_Add` (`self.AllFlags`) _array_element)))
  (for _array_element_2 (`self.AllFlags`)
    (bind _returnvalue (`KismetMathLibrary.VSize` (- (`self.K2_GetActorLocation` MyBot) (`self.K2_GetActorLocation` _array_element_2))))
    (if (< _returnvalue (`self.NearbyFlag`))
      (set `self.NearbyFlag` _returnvalue)
      (set `self.FlagTarget` _array_element_2)))
  (set `self.NearbyFlag` 9999999.0)
  (if true
    (`self.RunBehaviorTree` "/Game/Blueprints/AI/BotEnemyEasy_BehaviorTree.BotEnemyEasy_BehaviorTree")
    (else
      (`self.RunBehaviorTree` "/Game/Blueprints/AI/BotEnemyHard_BehaviorTree.BotEnemyHard_BehaviorTree")))
  (`BlackboardComponent.SetValueAsVector` (`AIBlueprintHelperLibrary.GetBlackboard` null) "TargetLocation" (+ (`self.K2_GetActorLocation` _flagtarget) (`/Game/Blueprints/FlagBlueprint.SpawnLocation` _flagtarget)))
  (set `self.FlagTarget` (`self.NullFlag`))
  (`KismetArrayLibrary.Array_Clear` (`self.AllFlags`))
  (`self.Ammo`))

(event `self.OnPossess`
  (params (PossessedPawn :type "Pawn Object Reference"))
  (bind _asbot_enemy (cast `BotEnemy` PossessedPawn :!pure true))
  (set `self.StoredPawn` _asbot_enemy)
  (`KismetArrayLibrary.Array_Add` (`self.ActorsToIgnore`) _asbot_enemy))

(event `self.ReceiveTick`
  (params (DeltaSeconds :type "Float (single-precision)"))
  (bind _storedpawn (`self.StoredPawn`))
  (bind _actorstoignore (`self.ActorsToIgnore`))
  (bind _returnvalue (`self.K2_GetActorLocation` _storedpawn))
  (if (and (>= (`KismetMathLibrary.VSize` (`self.GetVelocity` _storedpawn)) 50.0) (not (`Entity.GetIsAimBow` _storedpawn)))
    (if (>= (`Entity.GetSpeed` _storedpawn) 37.5)
      (set `self.SphereLength` 400.0)
      (else
        (set `self.SphereLength` 100.0)))
    (bind (_outhit _returnvalue_2) (`KismetSystemLibrary.SphereTraceSingle` _returnvalue (+ _returnvalue (* (`self.GetActorForwardVector` _storedpawn) (`self.SphereLength`))) 40.0 "TraceTypeQuery1" false (`self.ActorsToIgnore`) "None" true (struct :`R` 1.0 :`A` 1.0) (struct :`G` 1.0 :`A` 1.0) 0.0))
    (bind (_bblockinghit _binitialoverlap _time _distance _location _impactpoint _normal _impactnormal _physmat _hitactor) (`GameplayStatics.BreakHitResult` _outhit))
    (bind _asentity (cast `Entity` _hitactor)
      (:`then`
        (if (not (`KismetArrayLibrary.Array_Contains` _actorstoignore _asentity))
          (`KismetArrayLibrary.Array_Add` _actorstoignore _asentity)))
      (:`CastFailed`
        (bind _asweapon (cast `Weapon` _hitactor)
          (:`then`
            (if (not (`KismetArrayLibrary.Array_Contains` _actorstoignore _asweapon))
              (`KismetArrayLibrary.Array_Add` _actorstoignore _asweapon)))
          (:`CastFailed`
            (if _returnvalue_2
              (`Entity.JumpAnim` (`self.StoredPawn`)))))))))

(event `Die`
  (bind _actorstoignore (`self.ActorsToIgnore`))
  (bind _returnvalue (`AIBlueprintHelperLibrary.GetBlackboard` self))
  (`self.RunBehaviorTree` null)
  (`BlackboardComponent.SetValueAsBool` _returnvalue "CanSeeTarget" false)
  (`BlackboardComponent.SetValueAsBool` _returnvalue "HasAmmo" false)
  (`BlackboardComponent.SetValueAsBool` _returnvalue "IsNear" false)
  (`BlackboardComponent.SetValueAsBool` _returnvalue "IsCaptureFlag" false)
  (`KismetSystemLibrary.Delay` 6.0)
  (if true
    (`self.RunBehaviorTree` "/Game/Blueprints/AI/BotEnemyEasy_BehaviorTree.BotEnemyEasy_BehaviorTree")
    (else
      (`self.RunBehaviorTree` "/Game/Blueprints/AI/BotEnemyHard_BehaviorTree.BotEnemyHard_BehaviorTree")))
  (`self.BeginPlayBot` (cast `/Game/Blueprints/MyBotEnemy` (`self.StoredPawn`) :!pure true))
  (`KismetArrayLibrary.Array_Clear` _actorstoignore)
  (`KismetArrayLibrary.Array_Add` _actorstoignore (`self.StoredPawn`))
  (`self.Ammo`))

(event `Ammo`
  (`BlackboardComponent.SetValueAsBool` (`AIBlueprintHelperLibrary.GetBlackboard` self) "HasAmmo" (> (`Entity.GetAmmoArrow` (`self.StoredPawn`)) 0)))

(fn `UserConstructionScript`)